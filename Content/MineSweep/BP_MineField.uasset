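; Minesweeper field actor that lays out cells as a grid centered on itself.
; The construction script rebuilds an instanced preview of the grid from its width, length and cell width.
; When a cell is added, it attaches the cell to itself, places it by column and row, and sets its size.
; Preview and live cells share the same position functions, which space cells by their width plus a fixed gap.
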(event EventBeginPlay)

(event Collision|EventActorBeginOverlap
  (params (OtherActor :type Actor%20Object%20Reference)))

(event EventTick
  (params (DeltaSeconds :type Float%20%28single-precision%29)))

(event EventHandleCellAdded
  (params (NewCell :type Cell%20Object%20Reference))
  (Utilities|IsValid NewCell
    (:Is%20Valid
      (Class|MineField|UpdateCell NewCell))))

(event EventUpdateCell
  (params (CellToUpdate :type Cell%20Object%20Reference))
  (bind _cellwidth (Variables|Size|GetCellWidth))
  (Utilities|IsValid CellToUpdate
    (:Is%20Valid
      (Utilities|FlowControl|Sequence
        (:then_0
          (Transformation|AttachActorToActor CellToUpdate self "None" "SnapToTarget" "SnapToTarget" "SnapToTarget" false)
          (bind _result (CallFunction|GetPositionforCell CellToUpdate))
          (Transformation|SetActorRelativeLocation CellToUpdate _result false true))
        (:then_1
          (Class|Cell|SetCellSize CellToUpdate (Math|Vector2D|MakeVector2D _cellwidth _cellwidth)))))))

(fn ConstructionScript
  (bind _cellwidth (Variables|Size|GetCellWidth))
  (bind _returnvalue (/ _cellwidth 1e+02))
  (Utilities|FlowControl|Sequence
    (:then_0
      (Components|InstancedStaticMesh|ClearInstances (Variables|Default|GetCellsPreview))
      (bind (_row _column) (Utilities|ForLoop2D 0 (- (Variables|Default|GetLength) 1) 0 (- (Variables|Default|GetWidth) 1))
        (:LoopBody
          (bind _result (CallFunction|GetPositionforCellCoordinates _column _row))
          (Components|InstancedStaticMesh|AddInstance (Variables|Default|GetCellsPreview) (Math|Transform|MakeTransform _result "0, 0, 0" (Math|Vector|MakeVector _returnvalue _returnvalue 0.1))))))))

(fn GetCellOffset
  (params (Column :type Integer) (Row :type Integer))
  (return (* (- (Math|Vector2D|MakeVector2D (Math|Conversions|ToFloat(Integer) Column) (Math|Conversions|ToFloat(Integer) Row)) (/ (- (Math|Vector2D|MakeVector2D (Math|Conversions|ToFloat(Integer) (Variables|Default|GetWidth)) (Math|Conversions|ToFloat(Integer) (Variables|Default|GetLength))) 1.0) 2.0)) (CallFunction|GetCellSpacing))))

(fn GetPositionforCell
  (params (Cell :type Cell%20Object%20Reference))
  (bind _returnvalue (Class|MineField|GetCellCoordinates Cell))
  (bind _result (CallFunction|GetPositionforCellCoordinates (.column _returnvalue) (.row _returnvalue)))
  (return _result))

(fn GetPositionforCellCoordinates
  (params (Column :type Integer) (Row :type Integer))
  (bind _returnvalue (CallFunction|GetCellOffset Column Row))
  (return (Math|Conversions|ToVector(Vector2D) _returnvalue)))

(fn GetCellSpacing
  (return (+ (Variables|Size|GetCellWidth) 1e+01)))