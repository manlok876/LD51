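; BP_Bomb is a bomb actor for the MineSweep game that reports its lifetime and explosion to the game framework.
; It increments the bomb counter on BP_MineSweepGS at BeginPlay and decrements it at EndPlay, so the game state tracks live bombs.
; Its Explode event passes the bomb itself to BP_MineSweepGM's HandleBombExplosion, leaving the consequences to the game mode.
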(event EventBeginPlay
  (bind _asbp_mine_sweep_gs (Utilities|Casting|CastToBP_MineSweepGS (Game|GetGameState)))
  (Default|IncrementBombCounter _asbp_mine_sweep_gs))

(event Collision|EventActorBeginOverlap
  (params (OtherActor :type Actor%20Object%20Reference)))

(event EventTick
  (params (DeltaSeconds :type Float%20%28single-precision%29)))

(event EventExplode
  (bind _asbp_mine_sweep_gm (Utilities|Casting|CastToBP_MineSweepGM (Game|GetGameMode)))
  (Default|HandleBombExplosion _asbp_mine_sweep_gm self))

(event EventEndPlay
  (params (EndPlayReason :type EEndPlayReason%20Enum :default "Destroyed"))
  (bind _asbp_mine_sweep_gs (Utilities|Casting|CastToBP_MineSweepGS (Game|GetGameState)))
  (Default|DecrementBombCounter _asbp_mine_sweep_gs))

(fn ConstructionScript)