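; Game mode for a cyclic Minesweeper variant that keeps adding bombs to the mine field on a looping timer.
; Each cycle ages bombs under closed cells, clears flagged ones, spawns as many bombs as the cycle number and recounts neighbor counters.
; New bombs land randomly within a region, which is re-covered as a veil if open cells surround the bomb, masking its exact position.
; The first explosion reveals all bombs, stops cycles and shows the HUD lose message.
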(event Custom|LaunchCycles
  (params (Time :type Float%20%28single-precision%29))
  (bind _returnvalue (Utilities|Time|SetTimerbyEvent (delegate Custom|HandleCycleEnded) Time true))
  (bind _minesweepgs (Variables|Default|GetMineSweepGS)
    (:then
      (Variables|/Game/Game/BP_MineSweepGS.BP_MineSweepGS_C|SetCycleTimer _minesweepgs _returnvalue))
    (:else)))

(event Custom|StopCycles
  (bind _minesweepgs (Variables|Default|GetMineSweepGS)
    (:then
      (Utilities|Time|ClearandInvalidateTimerbyHandle (Variables|/Game/Game/BP_MineSweepGS.BP_MineSweepGS_C|GetCycleTimer _minesweepgs)))
    (:else)))

(event Custom|UpdateExistingBombs
  (bind _minefield (Variables|Default|GetMineField)
    (:then
      (bind _returnvalue (Class|MineField|GetAllBombCells _minefield))
      (for _array_element _returnvalue
        (switch Utilities|FlowControl|Switch|SwitchonECellState (Variables|/Script/LD51.Cell|GetState _array_element)
          (:ECS_Closed
            (bind _bomb (Variables|/Script/LD51.Cell|GetBomb _array_element)
              (:then
                (Class|Bomb|IncrementCycles _bomb))
              (:else)))
          (:ECS_Flag
            (Class|Cell|ClearBomb _array_element true)
            (Class|Cell|RemoveFlag _array_element)))))
    (:else)))

(event Custom|IncrementCyclesCounter
  (bind _minesweepgs (Variables|Default|GetMineSweepGS)
    (:then
      (Default|IncrementCyclesCounter _minesweepgs))
    (:else)))

(event Custom|ClearAllFlags
  (bind _minefield (Variables|Default|GetMineField)
    (:then
      (for _array_element (Class|MineField|GetAllCells _minefield)
        (Class|Cell|RemoveFlag _array_element)))
    (:else)))

(event Custom|HandleCycleEnded
  (Utilities|FlowControl|Sequence
    (:then_0
      (CallFunction|IncrementCyclesCounter))
    (:then_1
      (CallFunction|UpdateExistingBombs))
    (:then_2
      (bind _newbombs (CallFunction|GetBombCounttoSpawn))
      (CallFunction|SpawnBombs _newbombs))
    (:then_3
      (CallFunction|UpdateBombsCounters))
    (:then_4
      (Development|PrintString (Utilities|String|Append "Cycle " (Utilities|String|ToString(Integer) (CallFunction|GetCurrentCycleNumber)) " start")))))

(event Custom|HandleBombExplosion
  (params (Bomb :type BP%20Bomb%20Object%20Reference))
  ;[1 1 1] GameOver
  (Utilities|FlowControl|DoOnce false
    (:Completed
      (Utilities|FlowControl|Sequence
        (:then_0
          (CallFunction|ShowAllBombs))
        (:then_1
          (CallFunction|StopCycles))
        (:then_2
          (bind _foundwidgets (Class|WidgetBlueprintLibrary|GetAllWidgetswithInterface "/Game/UI/UI_HUD.UI_HUD_C" false))
          (Class|UIHUD|Lose(Message) _foundwidgets))))))

(event Custom|ShowAllBombs
  ;[1 1 1] GameOver
  (bind _minefield (Variables|Default|GetMineField)
    (:then
      (bind _returnvalue (Class|MineField|GetAllBombs _minefield))
      (for _array_element _returnvalue
        (Rendering|SetActorHiddenInGame _array_element false)))
    (:else)))

(event Custom|SpawnBombs
  (params (BombCount :type Integer))
  (Variables|Default|GetMineField
    (:then
      (for _index (range 1 BombCount)
        (bind _result (CallFunction|GetCoordsforNewBomb))
        (CallFunction|SpawnBomb _result))
      (CallFunction|UpdateBombsCounters))
    (:else)))

(event Custom|SpawnBombsInitial
  (params (BombCount :type Integer))
  (CallFunction|SpawnBombs BombCount))

(event Custom|UpdateBombsCounters
  (Utilities|FlowControl|Sequence
    (:then_0
      (CallFunction|ClearAllCounters))
    (:then_1
      (bind _minefield (Variables|Default|GetMineField)
        (:then
          (bind _returnvalue (Class|MineField|GetAllBombCoords _minefield))
          (for _array_element _returnvalue
            (bind _returnvalue_2 (Class|MineUtils|GetNeighboringCellsbyCoords _minefield _array_element false))
            (for _array_element_2 _returnvalue_2
              (Utilities|IsValid _array_element_2
                (:Is%20Valid
                  (Variables|/Script/LD51.Cell|SetBombsAround _array_element_2 (+ (Variables|/Script/LD51.Cell|GetBombsAround _array_element_2) 1)))))))
        (:else)))))

(event Custom|SpawnBomb
  (params (FieldCoords :type Grid%20Coords%20Structure))
  (bind _minefield (Variables|Default|GetMineField)
    (:then
      (bind _returnvalue (Class|MineUtils|GetRandomFieldCoordsinRegion _minefield FieldCoords (- (Variables|Default|GetVeilDiameter) 2)))
      (Utilities|FlowControl|Sequence
        (:then_0
          (if (CallFunction|ShouldSpawnVeilAroundBomb _returnvalue)
            (bind (_from _to) (Class|MineUtils|GetRegion FieldCoords (Variables|Default|GetVeilDiameter)))
            (bind _returnvalue_2 (Class|MineUtils|GetRegionCoords _from _to))
            (bind _returnvalue_3 (Class|MineUtils|FilterValidCoordsforField _minefield _returnvalue_2))
            (for _array_element _returnvalue_3
              (Utilities|IsValid (Class|MineField|GetCellbyCoords _minefield _array_element)
                (:Is%20Valid
                  (Class|Cell|CoverCell (Class|MineField|GetCellbyCoords _minefield _array_element)))))))
        (:then_1
          (Utilities|IsValid (Class|MineField|GetCellbyCoords _minefield _returnvalue)
            (:Is%20Valid
              (bind _returnvalue_4 (Game|SpawnActorfromClass "/Game/MineSweep/BP_Bomb.BP_Bomb_C" (Transformation|GetActorTransform (Class|MineField|GetCellbyCoords _minefield _returnvalue)) "Undefined" 0 0))
              (Class|Cell|PlantBomb (Class|MineField|GetCellbyCoords _minefield _returnvalue) _returnvalue_4))))))
    (:else)))

(event Custom|ClearAllCounters
  (bind _minefield (Variables|Default|GetMineField)
    (:then
      (for _array_element (Class|MineField|GetAllCells _minefield)
        (Utilities|IsValid _array_element
          (:Is%20Valid
            (Variables|/Script/LD51.Cell|SetBombsAround _array_element 0)))))
    (:else)))

(event EventBeginPlay
  (Utilities|FlowControl|Sequence
    (:then_0
      (bind _returnvalue (Actor|GetActorOfClass "/Game/MineSweep/BP_MineField.BP_MineField_C"))
      (Variables|Default|SetMineField _returnvalue))
    (:then_1
      (bind _asbp_mine_sweep_gs (Utilities|Casting|CastToBP_MineSweepGS (Game|GetGameState)))
      (Variables|Default|SetMineSweepGS _asbp_mine_sweep_gs))
    (:then_2
      (CallFunction|SpawnBombsInitial (Variables|Default|GetInitialBombs)))
    (:then_3
      (CallFunction|LaunchCycles (Variables|Default|GetCycleDuration)))))

(event EventTick
  (params (DeltaSeconds :type Float%20%28single-precision%29)))

(fn ConstructionScript)

(fn GetCoordsforNewBomb
  (bind _minefield (Variables|Default|GetMineField)
    (:then
      (bind _returnvalue (Class|MineUtils|GetRandomCoordsWithoutBomb _minefield))
      (return _returnvalue))
    (:else
      (return ""))))

(fn ShouldSpawnVeilAroundBomb
  (params (BombCoords :type Grid%20Coords%20Structure))
  (bind _minefield (Variables|Default|GetMineField)
    (:then
      (bind _returnvalue (Class|MineUtils|GetNeighboringCellsbyCoords _minefield BombCoords true))
      (for _array_element _returnvalue
        (if (CallFunction|ShouldVeilCell _array_element)
          (return true)))
      (return false))
    (:else
      (return false))))

(fn GetBombCounttoSpawn
  (return (CallFunction|GetCurrentCycleNumber)))

(fn GetCurrentCycleNumber
  (bind _minesweepgs (Variables|Default|GetMineSweepGS)
    (:then
      (return (Variables|/Game/Game/BP_MineSweepGS.BP_MineSweepGS_C|GetCyclesCounter _minesweepgs)))
    (:else
      (return 0))))

(fn ShouldVeilCell
  (params (Cell :type Cell%20Object%20Reference))
  (Utilities|IsValid Cell
    (:Is%20Valid
      (switch Utilities|FlowControl|Switch|SwitchonECellState (Variables|/Script/LD51.Cell|GetState Cell)
        (:ECS_Open
          (return true))
        (:ECS_Closed
          _)
        (:ECS_Flag
          _))
      (return false))))