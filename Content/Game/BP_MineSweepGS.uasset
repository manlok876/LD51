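; Game state for a Minesweeper-style game that tracks bombs, placed flags, elapsed cycles and a doomsday countdown.
; Simple events raise or lower the bomb and flag counters and increment the cycle count, and getters expose these values.
; Flag placement is allowed only while flags number fewer than bombs.
; Remaining cycle time comes from a timer handle; neither that timer nor the doomsday countdown is set in these graphs.
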(event Custom|IncrementCyclesCounter
  (Math|Integer|IncrementInt (Variables|Default|GetCyclesCounter)))

(event Custom|DecrementFlagsCounter
  (Math|Integer|DecrementInt (Variables|Default|GetFlagsCounter)))

(event Custom|IncrementFlagsCounter
  (Math|Integer|IncrementInt (Variables|Default|GetFlagsCounter)))

(event Custom|IncrementBombCounter
  (Math|Integer|IncrementInt (Variables|Default|GetBombCounter)))

(event Custom|DecrementBombCounter
  (Math|Integer|DecrementInt (Variables|Default|GetBombCounter)))

(event EventBeginPlay)

(event EventTick
  (params (DeltaSeconds :type Float%20%28single-precision%29)))

(fn ConstructionScript)

(fn GetCurrentBombCount
  (return (Variables|Default|GetBombCounter)))

(fn GetCycleTimeLeft
  (return (Utilities|Time|GetTimerRemainingTimebyHandle (Variables|Default|GetCycleTimer))))

(fn GetCurrentFlagCount
  (return (Variables|Default|GetFlagsCounter)))

(fn GetCyclesPassed
  (return (Variables|Default|GetCyclesCounter)))

(fn CanPlaceFlag
  (return (< (Variables|Default|GetFlagsCounter) (Variables|Default|GetBombCounter))))

(fn GetCyclesUntilDoomsday
  (return (Variables|Default|GetDoomsdayCountdown)))